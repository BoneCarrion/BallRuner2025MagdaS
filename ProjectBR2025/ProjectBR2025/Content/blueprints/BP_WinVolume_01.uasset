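; BP_WinVolume_01 is a level exit trigger that completes the level when its box is overlapped and no BP_Crystal01 actors remain.
; If crystals remain, it prints a Polish message that not all were collected.
; Completion finds the current level's name in the TabLevelNames01 array and opens the next entry, or prints a last-level message on the final one.
; The overlap does not check which actor entered.
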(event OnComponentBeginOverlap(Box)
  (params (OverlappedComponent :type Primitive%20Component%20Object%20Reference) (OtherActor :type Actor%20Object%20Reference) (OtherComp :type Primitive%20Component%20Object%20Reference) (OtherBodyIndex :type Integer) (bFromSweep :type Boolean) (SweepResult :type Hit%20Result%20Structure%20%28by%20ref%29))
  (bind _outactors (Actor|GetAllActorsOfClass "/Game/blueprints/BP_Crystal01.BP_Crystal01_C"))
  (if (> (Utilities|Array|Length _outactors) 0)
    (Development|PrintString "Nie zebrano wszystkich kryształów")
    (else
      (CallFunction|CompleteLevel))))

(fn ConstructionScript)

(fn GetCurrentlevelIndex
  (bind _returnvalue (Game|GetCurrentLevelName true))
  (return (Utilities|Array|FindItem (Variables|Default|Gettab_levelNames_01) _returnvalue)))

(fn GetNextlevelName
  (return (Utilities|Array|Get(acopy) (Variables|Default|Gettab_levelNames_01) (+ (CallFunction|GetCurrentlevelIndex) 1))))

(fn LoadNextlevel
  (Game|OpenLevel(byName) (Utilities|String|StringToName (CallFunction|GetNextlevelName))))

(fn IsFinalLevel
  (return (== (Utilities|Array|LastIndex (Variables|Default|Gettab_levelNames_01)) (CallFunction|GetCurrentlevelIndex))))

(fn CompleteLevel
  (if (CallFunction|IsFinalLevel)
    (Development|PrintString "To jest Ostatni Poziom")
    (else
      (CallFunction|LoadNextlevel))))