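; BP_ball01 is a player-controlled rolling ball that restarts the level when it takes any damage.
; Forward/back and left/right axis inputs share one AddTorque node on the Sphere, applied as an acceleration change scaled by StrMultiply.
; The screen fades in on BeginPlay; damage plays an "oof" sound, fades out, then reopens the current level after a short delay.
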(event Game|Damage|EventAnyDamage
  (params (Damage :type Float%20%28single-precision%29) (DamageType :type Damage%20Type%20Object%20Reference) (InstigatedBy :type Controller%20Object%20Reference) (DamageCauser :type Actor%20Object%20Reference))
  (Audio|PlaySound2D "/Game/sounds/Minecraft_Damage__Oof__-_Sound_Effect__HD___online-audio-converter_com_.Minecraft_Damage__Oof__-_Sound_Effect__HD___online-audio-converter_com_" 1.0 1.0 0.0 0 0)
  (CameraFades|StartCameraFade :self (Game|GetPlayerCameraManager 0) :ToAlpha 1.0 :Duration 1.5 :bHoldWhenFinished true)
  (Utilities|FlowControl|Delay 2.0)
  (bind _returnvalue (Game|GetCurrentLevelName true))
  (Game|OpenLevel(byName) (Utilities|String|StringToName _returnvalue)))

(event EventBeginPlay
  (CameraFades|StartCameraFade :self (Game|GetPlayerCameraManager 0) :FromAlpha 1.0 :Duration 2.0 :bHoldWhenFinished true))

(event Input|AxisEvents|InputAxisMoveForwardBack
  (params (AxisValue :type Float%20%28single-precision%29))
  (bind _str_multiply (Variables|Default|GetStr%20Multiply))
  (Class|PrimitiveComponent|AddTorqueinRadians (Variables|Default|GetSphere) (Math|Vector|MakeVector (* (stale Input|AxisEvents|InputAxisMoveLeftRight AxisValue) _str_multiply) (* AxisValue _str_multiply) 0.0) "None" true))

(event Input|AxisEvents|InputAxisMoveLeftRight
  (params (AxisValue :type Float%20%28single-precision%29))
  (bind _str_multiply (Variables|Default|GetStr%20Multiply))
  (Class|PrimitiveComponent|AddTorqueinRadians (Variables|Default|GetSphere) (Math|Vector|MakeVector (* AxisValue _str_multiply) (* (stale Input|AxisEvents|InputAxisMoveForwardBack AxisValue) _str_multiply) 0.0) "None" true))

(fn ConstructionScript)